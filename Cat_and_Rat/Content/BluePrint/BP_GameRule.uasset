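; BP_GameRule runs the match rules for a cats-versus-rats game, handling the countdown, HUD, music and game over.
; On BeginPlay it starts a one-second timer, shows the in-game UI and binds messiness and win callbacks from the C++ TagAgentSubsystem.
; A cat win, rat win or expired timer, which counts as a cat win, triggers a one-shot GameOver that shows the result screen and pauses.
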(event Custom|Update_timer
  ;[0.15 0.15 0.15 0.5] 타이머
  ;;[0.15 0.15 0.15 0.5] 시간 계산
  (bind _output_get (Variables|Default|SetCurrnetTime (- (Variables|Default|GetCurrnetTime) 1.0)))
  (if (<= _output_get 0.0)
    (CallFunction|GameOver true)))

(event Custom|GameOver
  (params (bCatWin :type Boolean))
  (bind _returnvalue (Game|GetPlayerController 0))
  ;[0.15 0.15 0.15 0.5] GameOver
  (if (not (Variables|Default|GetbIsGameOver))
    (Variables|Default|SetbIsGameOver true)
    ;[0.15 0.15 0.15 0.5] 타이머
    (Utilities|Time|ClearandInvalidateTimerbyHandle (stale EventBeginPlay _returnvalue_2))
    (Viewport|RemoveAllWidgets)
    ;[0.15 0.15 0.15 0.5] 게임오버 UI 생성
    (Audio|Components|Audio|Stop (Variables|Default|GetMainBGM))
    (bind _returnvalue_2 (UserInterface|CreateWidget "/Game/UI/GameOver_UI.GameOver_UI_C" 0 bCatWin))
    (UserInterface|Viewport|AddtoViewport _returnvalue_2 0)
    (Variables|/Script/Engine.PlayerController|SetbShowMouseCursor _returnvalue true)
    (Input|SetInputModeUIOnly _returnvalue _returnvalue_2 "DoNotLock" false)
    (Game|SetGamePaused true)))

(event Custom|OnCatsWin
  ;[0.15 0.15 0.15 0.5] C++코드와 연결 승, 패 처리 및 어지러움 수치 바인딩
  (CallFunction|GameOver true))

(event Custom|OnRatsWin
  ;[0.15 0.15 0.15 0.5] C++코드와 연결 승, 패 처리 및 어지러움 수치 바인딩
  (CallFunction|GameOver false))

(event Custom|OnMessinessChanged
  (params (Percent :type Float%20%28single-precision%29))
  ;[0.15 0.15 0.15 0.5] C++코드와 연결 승, 패 처리 및 어지러움 수치 바인딩
  (Variables|Default|SetCurrentMessiness Percent))

(event EventBeginPlay
  (bind _returnvalue (Subsystems|GetTagAgentSubsystem))
  ;[0.15 0.15 0.15 0.5] 타이머
  (bind _returnvalue_2 (Utilities|Time|SetTimerbyEvent (delegate Custom|Update_timer) 1.0 true))
  ;[0.15 0.15 0.15 0.5] InGame UI 생성
  (bind _returnvalue_3 (UserInterface|CreateWidget "/Game/UI/InGame_UI.InGame_UI_C"))
  (UserInterface|Viewport|AddtoViewport _returnvalue_3 5)
  ;;[0.15 0.15 0.15 0.5] 상단 ui 인원 수 따라
  (Default|UpdateTeamUI _returnvalue_3 (Variables|Default|GetCurrentCatCount) (Variables|Default|GetCurrentMouseCount))
  ;[0.15 0.15 0.15 0.5] C++코드와 연결 승, 패 처리 및 어지러움 수치 바인딩
  (EventDispatchers|AssignOnMessinessChanged _returnvalue (delegate Custom|OnMessinessChanged))
  (EventDispatchers|AssignOnCatsWin _returnvalue (delegate Custom|OnCatsWin))
  (EventDispatchers|AssignOnRatsWin _returnvalue (delegate Custom|OnRatsWin))
  (bind _returnvalue_4 (Audio|SpawnSound2D "/Game/sound/sound_mainbgm.sound_mainbgm" 1.0 1.0 0.0 0))
  (Variables|Default|SetMainBGM _returnvalue_4))

(fn ConstructionScript)
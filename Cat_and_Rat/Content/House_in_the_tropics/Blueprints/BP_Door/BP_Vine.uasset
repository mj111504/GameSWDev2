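; BP_Vine is an interactive sliding component, named Door, that the player opens and closes from inside a trigger box.
; Overlapping the box enables player 0's input on the actor, and leaving it disables that input.
; E or left mouse drives a FlipFlop that alternately plays and reverses a timeline, lerping Door's relative Y position between closed and offset.
; The opening branch also disables and immediately re-enables input.
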(event OnComponentBeginOverlap(Box)
  (params (OverlappedComponent :type Primitive%20Component%20Object%20Reference) (OtherActor :type Actor%20Object%20Reference) (OtherComp :type Primitive%20Component%20Object%20Reference) (OtherBodyIndex :type Integer) (bFromSweep :type Boolean) (SweepResult :type Hit%20Result%20Structure%20%28by%20ref%29))
  (Input|EnableInput (Game|GetPlayerController 0)))

(event OnComponentEndOverlap(Box)
  (params (OverlappedComponent :type Primitive%20Component%20Object%20Reference) (OtherActor :type Actor%20Object%20Reference) (OtherComp :type Primitive%20Component%20Object%20Reference) (OtherBodyIndex :type Integer))
  (Input|DisableInput (Game|GetPlayerController 0)))

(event Input|KeyboardEvents|E
  (params (Key :type Key%20Structure))
  (bind _returnvalue (Game|GetPlayerController 0))
  (:Pressed
    (if true
      (Utilities|FlowControl|FlipFlop
        (:A
          (Utilities|FlowControl|Sequence
            (:then_0
              (Input|DisableInput _returnvalue)
              (Input|EnableInput _returnvalue))
            (:then_1
              (bind _newtrack_0 (Timeline|Timeline_0 Play)
                (:Update
                  (Transformation|SetRelativeLocation (Variables|Default|GetDoor) (Math|Vector|MakeVector 0.0 (Math|Float|Lerp 0.0 7e+01 _newtrack_0) 0.0) false false))))))
        (:B
          (Utilities|FlowControl|Sequence
            (:then_0
              (Timeline|Timeline_0 Reverse))))))))

(event Input|MouseEvents|LeftMouseButton
  (params (Key :type Key%20Structure))
  (bind _returnvalue (Game|GetPlayerController 0))
  (:Pressed
    (if true
      (Utilities|FlowControl|FlipFlop
        (:A
          (Utilities|FlowControl|Sequence
            (:then_0
              (Input|DisableInput _returnvalue)
              (Input|EnableInput _returnvalue))
            (:then_1
              (bind _newtrack_0 (Timeline|Timeline_0 Play)
                (:Update
                  (Transformation|SetRelativeLocation (Variables|Default|GetDoor) (Math|Vector|MakeVector 0.0 (Math|Float|Lerp 0.0 7e+01 _newtrack_0) 0.0) false false))))))
        (:B
          (Utilities|FlowControl|Sequence
            (:then_0
              (Timeline|Timeline_0 Reverse))))))))

(fn ConstructionScript)
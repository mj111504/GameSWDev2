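; Interactive glass door that the player swings open and closed while standing inside its trigger box.
; Box overlap enables and disables input from player controller 0, and E or left mouse button drives a FlipFlop.
; The DoorRotation timeline plays or reverses to set the door's relative yaw.
; Each toggle plays a 2D open or close sound and briefly disables input as an animation cooldown.
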(event OnComponentBeginOverlap(Box)
  (params (OverlappedComponent :type Primitive%20Component%20Object%20Reference) (OtherActor :type Actor%20Object%20Reference) (OtherComp :type Primitive%20Component%20Object%20Reference) (OtherBodyIndex :type Integer) (bFromSweep :type Boolean) (SweepResult :type Hit%20Result%20Structure%20%28by%20ref%29))
  (Input|EnableInput (Game|GetPlayerController 0)))

(event OnComponentEndOverlap(Box)
  (params (OverlappedComponent :type Primitive%20Component%20Object%20Reference) (OtherActor :type Actor%20Object%20Reference) (OtherComp :type Primitive%20Component%20Object%20Reference) (OtherBodyIndex :type Integer))
  (Input|DisableInput (Game|GetPlayerController 0)))

(event Input|KeyboardEvents|E
  (params (Key :type Key%20Structure))
  (bind _returnvalue (Game|GetPlayerController 0))
  (:Pressed
    (if true
      (Utilities|FlowControl|FlipFlop
        (:A
          (Utilities|FlowControl|Sequence
            (:then_0
              ;[1 1 1] Звук открытия и закрытия двери
              (Audio|PlaySound2D "/Game/House_in_the_tropics/Blueprints/BP_Door/sound/DoorOpen.DoorOpen" 1.0 1.0 0.0 0 0)
              (Input|DisableInput _returnvalue)
              ;[1 1 1] Задержка анимации
              (Utilities|FlowControl|Delay 0.2)
              (Input|EnableInput _returnvalue))
            (:then_1
              (bind _rotation (Timeline|DoorRotation Play)
                (:Update
                  (Transformation|SetRelativeRotation (Variables|Default|GetDoor) (Math|Rotator|MakeRotator 0.0 0.0 _rotation) false false))))))
        (:B
          (Utilities|FlowControl|Sequence
            (:then_0
              (Timeline|DoorRotation Reverse))
            (:then_1
              (Audio|PlaySound2D "/Game/House_in_the_tropics/Blueprints/BP_Door/sound/DoorClosse.DoorClosse" 1.0 1.0 0.0 0 0)
              (Input|DisableInput _returnvalue)
              (Utilities|FlowControl|Delay 0.2)
              (Input|EnableInput _returnvalue))))))))

(event Input|MouseEvents|LeftMouseButton
  (params (Key :type Key%20Structure))
  (bind _returnvalue (Game|GetPlayerController 0))
  (:Pressed
    (if true
      (Utilities|FlowControl|FlipFlop
        (:A
          (Utilities|FlowControl|Sequence
            (:then_0
              ;[1 1 1] Звук открытия и закрытия двери
              (Audio|PlaySound2D "/Game/House_in_the_tropics/Blueprints/BP_Door/sound/DoorOpen.DoorOpen" 1.0 1.0 0.0 0 0)
              (Input|DisableInput _returnvalue)
              ;[1 1 1] Задержка анимации
              (Utilities|FlowControl|Delay 0.2)
              (Input|EnableInput _returnvalue))
            (:then_1
              (bind _rotation (Timeline|DoorRotation Play)
                (:Update
                  (Transformation|SetRelativeRotation (Variables|Default|GetDoor) (Math|Rotator|MakeRotator 0.0 0.0 _rotation) false false))))))
        (:B
          (Utilities|FlowControl|Sequence
            (:then_0
              (Timeline|DoorRotation Reverse))
            (:then_1
              (Audio|PlaySound2D "/Game/House_in_the_tropics/Blueprints/BP_Door/sound/DoorClosse.DoorClosse" 1.0 1.0 0.0 0 0)
              (Input|DisableInput _returnvalue)
              (Utilities|FlowControl|Delay 0.2)
              (Input|EnableInput _returnvalue))))))))

(fn ConstructionScript)
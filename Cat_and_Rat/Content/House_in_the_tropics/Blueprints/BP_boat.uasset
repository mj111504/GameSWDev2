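; Boat actor in the tropics house scene that rocks its static mesh using a timeline.
; BeginPlay enters a FlipFlop that, after short delays, alternately plays and reverses the timeline, which drives equal roll and pitch.
; The timeline update loops back into the FlipFlop through an always-true branch, keeping the cycle going.
; Each path also disables the actor's player input before its delay and re-enables it afterwards.
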(event EventBeginPlay
  (bind _returnvalue (Game|GetPlayerController 0))
  (if true :!label _label
    (Utilities|FlowControl|FlipFlop
      (:A
        (Utilities|FlowControl|Sequence
          (:then_0
            (Input|DisableInput _returnvalue)
            (Utilities|FlowControl|Delay 2.0)
            (Input|EnableInput _returnvalue)
            (bind _rotation (Timeline|Timeline_0 Play)
              (:Update
                (Transformation|SetRelativeRotation (Variables|Default|GetStaticMesh) (Math|Rotator|MakeRotator _rotation _rotation 0.0) false false)
                (goto _label))))))
      (:B
        (Utilities|FlowControl|Sequence
          (:then_1
            (Input|DisableInput _returnvalue)
            (Utilities|FlowControl|Delay 3.0)
            (Input|EnableInput _returnvalue)
            (Timeline|Timeline_0 Reverse)))))))

(fn ConstructionScript)